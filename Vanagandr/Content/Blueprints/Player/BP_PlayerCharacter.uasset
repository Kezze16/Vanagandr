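; Player character Blueprint that adds a horizontal speed cap on top of a PBPlayerMovement component and shows a quit-game button.
; BeginPlay caches the component's AxisSpeedLimit and, for locally controlled players, adds the WBP_QuitGameButton widget to the viewport.
; On authority only, Tick checks full 3D speed against that limit, then clamps X/Y velocity while preserving Z.
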(event EventBeginPlay
  (bind _aspbplayer_movement (Utilities|Casting|CastToPBPlayerMovement (Variables|Character|GetCharacterMovement)))
  (Variables|Default|SetAxis%20Speed%20Limit%20Bp (Variables|/Script/PBCharacterMovement.PBPlayerMovement|GetAxisSpeedLimit _aspbplayer_movement))
  (if (Pawn|IsLocallyControlled)
    (bind _returnvalue (UserInterface|CreateWidget "/Game/Blueprints/UI/WBP_QuitGameButton.WBP_QuitGameButton_C" (Class|GameplayStatics|GetPlayerControllerfromID)))
    (UserInterface|Viewport|AddtoViewport _returnvalue 0)))

(event EventTick
  (params (DeltaSeconds :type Float%20%28single-precision%29))
  (bind _returnvalue (Transformation|GetVelocity))
  (bind _charactermovement (Variables|Character|GetCharacterMovement))
  (bind _axis_speed_limit_bp (Variables|Default|GetAxis%20Speed%20Limit%20Bp))
  (bind _returnvalue_2 (Math|Vector|ClampVectorSize (Math|Vector|MakeVector (.x _returnvalue) (.y _returnvalue) 0.0) -999999999999.0 _axis_speed_limit_bp))
  ;[0.9564 1 0.6266] Speed Limit
  (if (Ability|HasAuthority)
    (if (> (Math|Vector|VectorLength (Variables|/Script/Engine.MovementComponent|GetVelocity _charactermovement)) (Variables|Default|GetAxis%20Speed%20Limit%20Bp))
      (Variables|/Script/Engine.MovementComponent|SetVelocity _charactermovement (Math|Vector|MakeVector (.x _returnvalue_2) (.y _returnvalue_2) (.z _returnvalue))))))

(fn ConstructionScript)