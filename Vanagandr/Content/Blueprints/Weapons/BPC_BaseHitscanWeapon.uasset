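; Base hitscan weapon component that adds a crosshair and fires on IA_Fire in single or timer-looped automatic mode.
; Each shot plays a sound and line-traces from the camera, with only debug drawing and printing of the hit actor, no damage.
; Tick-driven recoil applies a vector curve to control rotation while separating out player aim input, then interpolates back toward the starting rotation once firing stops.
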(event Input|EnhancedActionEvents|EnhancedInputActionIA_Fire
  (params (ActionValue :type Boolean) (ElapsedSeconds :type Float%20%28double-precision%29) (TriggeredSeconds :type Float%20%28double-precision%29) (InputAction :type Input%20Action%20Object%20Reference :default "/Game/Blueprints/Inputs/IA_Fire.IA_Fire"))
  (:Started
    (switch Utilities|FlowControl|Switch|SwitchonE_FirePattern (Variables|Default|GetFireMode)
      (:NewEnumerator0
        (Utilities|AutomaticFire))
      (:NewEnumerator2
        (Utilities|SingleFire))))
  (:Canceled
    (switch Utilities|FlowControl|Switch|SwitchonE_FirePattern (Variables|Default|GetFireMode) :!label _label
      (:NewEnumerator0
        (Utilities|Time|ClearandInvalidateTimerbyHandle (Variables|Default|GetAutomaticFireTimer)))
      (:NewEnumerator2
        _))
    (CallFunction|RecoilEnd))
  (:Completed
    (goto _label)))

(event EventTick
  (params (DeltaSeconds :type Float%20%28single-precision%29))
  (CallFunction|RecoilTick DeltaSeconds))

(event EventBeginPlay
  (bind _returnvalue (UserInterface|CreateWidget "/Game/Blueprints/UI/WBP_Crosshair.WBP_Crosshair_C"))
  (bind _output_get (Variables|Default|SetWidgetCrosshair _returnvalue))
  (UserInterface|Viewport|AddtoViewport _output_get 0))

(fn Fire
  (bind _returnvalue (Game|GetPlayerController 0))
  (bind _playercameramanager (Variables|/Script/Engine.PlayerController|GetPlayerCameraManager _returnvalue))
  (bind _rootcomponent (Variables|/Script/Engine.Actor|GetRootComponent _playercameramanager))
  (bind _returnvalue_2 (Transformation|GetWorldLocation _rootcomponent))
  (CallFunction|RecoilStart)
  (Audio|PlaySound2D "/Game/StarterContent/Audio/Explosion_Cue.Explosion_Cue" 1.0 1.0 0.0 0 0)
  (bind _outhit (Collision|LineTraceByChannel _returnvalue_2 (+ _returnvalue_2 (* (Math|Vector|GetForwardVector (Variables|/Script/Engine.Actor|GetRootComponent _playercameramanager)) (Variables|Default|GetActiveWeaponRange))) "TraceTypeQuery1" false 0 "Persistent"))
  (Utilities|IsValid (.HitActor (Collision|BreakHitResult _outhit))
    (:Is%20Valid
      (Development|PrintString (Utilities|GetDisplayName (.HitActor (Collision|BreakHitResult _outhit)))))))

(fn RecoilStart
  (Utilities|IsValid (Variables|Default|GetRecoilCurve)
    (:Is%20Valid
      (Variables|Default|SetPlayerDeltaRotation "0, 0, 0")
      (Variables|Default|SetRecoilDeltaRotation "0, 0, 0")
      (Variables|Default|SetDeltaRot "0, 0, 0")
      (Variables|Default|SetRecoilStartRotation (Pawn|GetControlRotation (Game|GetPlayerController 0) :!class /Script/Engine.Controller))
      (Variables|Default|SetisFiring? true)
      (bind _returnvalue (Utilities|Time|SetTimerbyFunctionName 0 "RecoilTimerFunction" 1e+01))
      (Variables|Default|SetRecoilDurationTimer _returnvalue)
      (Variables|Default|SetisAddingRecoil? true)
      (Variables|Default|SetisRecoveringFromRecoil? false))))

(fn RecoilEnd
  (Variables|Default|SetisFiring? false))

(fn RecoilTimerFunction
  (Variables|Default|SetisAddingRecoil? false))

(fn RecoilStartRecovering
  (if (> (.pitch (Pawn|GetControlRotation (Game|GetPlayerController 0) :!class /Script/Engine.Controller)) (.pitch (Variables|Default|GetRecoilStartRotation)))
    (Variables|Default|SetisRecoveringFromRecoil? true)
    (bind _returnvalue (Utilities|Time|SetTimerbyFunctionName 0 "RecoilTimerFunction" (Variables|Default|GetRecoilRecoveryTime)))
    (Variables|Default|SetRecoveryDurationTimer _returnvalue)))

(fn RecoveryTimerFunction
  (Variables|Default|SetisRecoveringFromRecoil? false))

(fn RecoilTick
  (params (Delta%20Seconds :type Float%20%28double-precision%29))
  (bind _returnvalue (Game|GetPlayerController 0))
  (bind _returnvalue_2 (Game|GetPlayerController 0))
  (bind _returnvalue_3 (Game|GetPlayerController 0))
  (bind _recoilstartrotation (Variables|Default|GetRecoilStartRotation))
  (bind _recoilstartrotation_2 (Variables|Default|GetRecoilStartRotation))
  (bind _returnvalue_4 (Pawn|GetControlRotation _returnvalue :!class /Script/Engine.Controller))
  (bind _returnvalue_5 (Pawn|GetControlRotation _returnvalue_3 :!class /Script/Engine.Controller))
  (bind _returnvalue_6 (Pawn|GetControlRotation _returnvalue_2 :!class /Script/Engine.Controller))
  (LocalVariables|SetDeltaTime Delta%20Seconds)
  (if (Variables|Default|GetisAddingRecoil?)
    (bind _output_get (LocalVariables|SetRecoilTimeElapsed (Class|KismetSystemLibrary|GetTimerElapsedTimeHandle (Variables|Default|GetRecoilDurationTimer))))
    (bind _output_get_2 (LocalVariables|SetRecoilVectorValue (Math|Curves|GetVectorValue (Variables|Default|GetRecoilCurve) _output_get)))
    (Variables|Default|SetDeltaRot (Math|Rotator|MakeRotator 0.0 (.y _output_get_2) (.z _output_get_2)))
    (bind _output_get_3 (Variables|Default|SetPlayerDeltaRotation (Math|Rotator|MakeRotator 0.0 (- (- (.pitch _returnvalue_4) (.pitch _recoilstartrotation)) (.pitch (Variables|Default|GetRecoilDeltaRotation))) (- (- (.yaw _returnvalue_4) (.yaw _recoilstartrotation)) (.yaw (Variables|Default|GetRecoilDeltaRotation))))))
    (Pawn|SetControlRotation (Game|GetPlayerController 0) (Math|Rotator|MakeRotator 0.0 (+ (.pitch _output_get_3) (.pitch _recoilstartrotation_2) (.pitch (Variables|Default|GetDeltaRot))) (+ (.yaw _output_get_3) (.yaw _recoilstartrotation_2) (.yaw (Variables|Default|GetDeltaRot)))))
    (Variables|Default|SetRecoilDeltaRotation (Variables|Default|GetDeltaRot))
    (if (not (Variables|Default|GetisFiring?))
      (if (> (Class|KismetSystemLibrary|GetTimerElapsedTimeHandle (Variables|Default|GetRecoilDurationTimer)) (Variables|Default|GetFireRate))
        (Variables|Default|SetisAddingRecoil? false)
        (CallFunction|RecoilEnd)
        (CallFunction|RecoilStartRecovering)))
    (elif (Variables|Default|GetisRecoveringFromRecoil?)
      (bind _output_get_4 (LocalVariables|SetTempRot (Pawn|GetControlRotation (Game|GetPlayerController 0) :!class /Script/Engine.Controller)))
      (if (> (.pitch _output_get_4) (.pitch (Variables|Default|GetRecoilStartRotation)))
        (Pawn|SetControlRotation (Game|GetPlayerController 0) (Math|Interpolation|RInterpTo (Pawn|GetControlRotation _returnvalue_2 :!class /Script/Engine.Controller) (Math|Rotator|MakeRotator 0.0 (- (.pitch _returnvalue_6) (.pitch (Variables|Default|GetRecoilDeltaRotation))) (- (.yaw _returnvalue_6) (.yaw (Variables|Default|GetRecoilDeltaRotation)))) (LocalVariables|GetDeltaTime) (Variables|Default|GetRecoilRecoverySpeed)))
        (Variables|Default|SetRecoilDeltaRotation (Math|Rotator|MakeRotator 0.0 (+ (.pitch (Variables|Default|GetRecoilDeltaRotation)) (- (.pitch _returnvalue_5) (.pitch (LocalVariables|GetTempRot)))) (+ (.yaw (Variables|Default|GetRecoilDeltaRotation)) (- (.yaw _returnvalue_5) (.yaw (LocalVariables|GetTempRot))))))
        (else
          (Utilities|Time|ClearandInvalidateTimerbyHandle (Variables|Default|GetRecoveryDurationTimer)))))))